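; BP_BirdsEyePlayerController is the bird's-eye player controller, handling structure building and tile inspection.
; BuildStructure shows a preview through BPBuildComponent and turns on build mode.
; The apply input builds and exits the mode on success, while abort hides the preview and exits.
; Tile selection changes replace the W_StructureInfo widget, showing one only when the selected tile has a valid structure.
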(event `self.BuildStructure`
  (params (StructureData :type "StructureData Structure (by ref)"))
  ;[1 1 1] Buildmode
  (`BuildComponent.ShowPreview` (`self.BP_BuildComponent`) StructureData)
  (`self.ToggleBuildMode` true))

(event `EnhancedInput|/Game/Input/Actions/IA_BuildApply`
  (params (ActionValue :type Boolean) (ElapsedSeconds :type "Float (double-precision)") (TriggeredSeconds :type "Float (double-precision)") (InputAction :type "InputAction Object Reference" :default "/Game/Input/Actions/IA_BuildApply.IA_BuildApply"))
  ;[1 1 1] Buildmode
  (:`Triggered`
    (bind _returnvalue (`BuildComponent.BuildStructure` (`self.BP_BuildComponent`)))
    (if _returnvalue
      (`self.ToggleBuildMode` false :!label _label))))

(event `EnhancedInput|/Game/Input/Actions/IA_BuildAbort`
  (params (ActionValue :type Boolean) (ElapsedSeconds :type "Float (double-precision)") (TriggeredSeconds :type "Float (double-precision)") (InputAction :type "InputAction Object Reference" :default "/Game/Input/Actions/IA_BuildAbort.IA_BuildAbort"))
  ;[1 1 1] Buildmode
  (:`Triggered`
    (`BuildComponent.HidePreview` (`self.BP_BuildComponent`))
    (goto _label)))

(event `self.TileSelectionChanged`
  (params (Tile :type "Tile Object Reference"))
  (bind _structure (`Tile.Structure` Tile))
  (bind _structureinfowidget (`self.StructureInfoWidget`))
  ;[1 1 1] Display structure info
  (`/Engine/EditorBlueprintResources/StandardMacros.IsValid` _structureinfowidget
    (:`Is Valid`
      (`Widget.RemoveFromParent` _structureinfowidget))
    (:`Is Not Valid`
      _))
  (`/Engine/EditorBlueprintResources/StandardMacros.IsValid` Tile
    (:`Is Valid`
      (`/Engine/EditorBlueprintResources/StandardMacros.IsValid` _structure
        (:`Is Valid`
          (bind _returnvalue (`|CreateWidget` "/Game/UI/StructureDataWidgets/W_StructureInfo.W_StructureInfo_C" null _structure))
          (bind _output_get (set `self.StructureInfoWidget` _returnvalue))
          (`UserWidget.AddToViewport` _output_get 0))))))

(fn `UserConstructionScript`)