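; Building component that previews and places data-table structures on the tile under the birds-eye player controller's cursor.
; BeginPlay loads structure rows, and ShowPreview adds a mesh to the owner for the selected one.
; UpdatePreview, repeatable through the self-calling BuildDelay timer, moves the mesh and tints it blue or red by tile structure and foundation checks.
; BuildStructure spawns the actor on valid tiles, registers it with the tile, and always hides the preview.
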(event `self.ReceiveBeginPlay`
  (bind _datatable (`self.DataTable`))
  (bind _outrownames (`DataTableFunctionLibrary.GetDataTableRowNames` _datatable))
  (for _array_element _outrownames
    (bind _returnvalue (`|GetDataTableRow` _datatable _array_element)
      (:`then`
        (`KismetArrayLibrary.Array_Add` (`self.StructureData`) _returnvalue)))))

(event `ShowPreview`
  (params (StructureID :type Integer))
  (bind (_output_structureclass _output_mesh) (break `/Game/Blueprints/Structures/DataTables/S_BPStructureData` (`|GetArrayItem` (`self.StructureData`) (`self.CurrentStructureID`))))
  (set `self.CurrentStructureID` StructureID)
  (set `self.BuildMode` true)
  (bind _returnvalue (`|AddComponentByClass` :`self` (`self.GetOwner`) :`Class` "/Script/Engine.StaticMeshComponent"))
  (bind _output_get (set `self.PreviewMesh` _returnvalue))
  (`StaticMeshComponent.SetStaticMesh` _output_get _output_mesh)
  (`self.UpdatePreview`))

(event `HidePreview`
  (set `self.BuildMode` false)
  (`self.K2_DestroyComponent` (`self.PreviewMesh`)))

(event `BuildStructure`
  (bind _output_structureclass (break `/Game/Blueprints/Structures/DataTables/S_BPStructureData` (`|GetArrayItem` (`self.StructureData`) (`self.CurrentStructureID`))))
  (bind _asbp_birds_eye_player_controller (cast `/Game/Blueprints/BP_BirdsEyePlayerController` (`GameplayStatics.GetPlayerController` 0)))
  (bind _returnvalue (`BirdsEyePlayerController.QueryTileUnderCursor` _asbp_birds_eye_player_controller))
  (if (`self.IsBuildLocationValid` _returnvalue)
    (bind _returnvalue_2 (`|SpawnActorFromClass` _output_structureclass (`KismetMathLibrary.MakeTransform` (`Tile.GetCenterSocketLocation` _returnvalue) (`SceneComponent.K2_GetComponentRotation` (`self.PreviewMesh`))) "Undefined" "OverrideRootScale" null null))
    (`Tile.Build` _returnvalue _returnvalue_2)
    (`self.HidePreview`)
    (else
      (`self.HidePreview`))))

(event `BuildDelay`
  (if (`self.BuildMode`)
    (`self.UpdatePreview`)
    (`KismetSystemLibrary.Delay` 0.1)
    (`self.BuildDelay`)))

(fn `IsBuildLocationValid`
  (params (Tile :type "Tile Object Reference"))
  (returns (isValid :type Boolean))
  (bind (_output_structureclass _output_mesh _output_supportedfoundationtypes) (break `/Game/Blueprints/Structures/DataTables/S_BPStructureData` (`|GetArrayItem` (`self.StructureData`) (`self.CurrentStructureID`))))
  (`/Engine/EditorBlueprintResources/StandardMacros.IsValid` Tile
    (:`Is Valid`
      (return (and (`KismetSystemLibrary.IsValid` (`Tile.Structure` Tile)) (`KismetArrayLibrary.Array_Contains` _output_supportedfoundationtypes (`Tile.TileFoundationType` Tile)))))
    (:`Is Not Valid`
      (return false))))

(fn `SetPreviewColor`
  (params (IsValidLocation :type Boolean))
  (bind _previewmesh (`self.PreviewMesh`))
  (for _index (range (`PrimitiveComponent.GetNumMaterials` _previewmesh))
    (if IsValidLocation
      (`PrimitiveComponent.SetMaterial` _previewmesh _index "/Game/Materials/M_PreviewBlue.M_PreviewBlue")
      (else
        (`PrimitiveComponent.SetMaterial` _previewmesh _index "/Game/Materials/M_PreviewRed.M_PreviewRed")))))

(fn `UpdatePreview`
  (bind _asbp_birds_eye_player_controller (cast `/Game/Blueprints/BP_BirdsEyePlayerController` (`GameplayStatics.GetPlayerController` 0)))
  (bind _returnvalue (`BirdsEyePlayerController.QueryTileUnderCursor` _asbp_birds_eye_player_controller))
  (`/Engine/EditorBlueprintResources/StandardMacros.IsValid` _returnvalue
    (:`Is Valid`
      (`self.SetPreviewColor` (`self.IsBuildLocationValid` _returnvalue))
      (`SceneComponent.K2_SetWorldLocation` (`self.PreviewMesh`) (`Tile.GetCenterSocketLocation` _returnvalue) false false))))