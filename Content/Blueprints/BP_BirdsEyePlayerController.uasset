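; Bird's-eye player controller that drives a build mode for placing structures through its build component.
; A BuildStructure event shows a preview for the given structure ID and switches build mode on.
; The apply input asks the component to build and leaves build mode only on success, while the abort input hides the preview and exits build mode.
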(event `self.BuildStructure`
  (params (StructureID :type Integer))
  ;[1 1 1] Buildmode
  (`BuildComponent.ShowPreview` (`self.BP_BuildComponent`) StructureID)
  (`self.ToggleBuildMode` true))

(event `EnhancedInput|/Game/Input/Actions/IA_BuildApply`
  (params (ActionValue :type Boolean) (ElapsedSeconds :type "Float (double-precision)") (TriggeredSeconds :type "Float (double-precision)") (InputAction :type "InputAction Object Reference" :default "/Game/Input/Actions/IA_BuildApply.IA_BuildApply"))
  ;[1 1 1] Buildmode
  (:`Triggered`
    (bind _returnvalue (`BuildComponent.BuildStructure` (`self.BP_BuildComponent`)))
    (if _returnvalue
      (`self.ToggleBuildMode` false :!label _label))))

(event `EnhancedInput|/Game/Input/Actions/IA_BuildAbort`
  (params (ActionValue :type Boolean) (ElapsedSeconds :type "Float (double-precision)") (TriggeredSeconds :type "Float (double-precision)") (InputAction :type "InputAction Object Reference" :default "/Game/Input/Actions/IA_BuildAbort.IA_BuildAbort"))
  ;[1 1 1] Buildmode
  (:`Triggered`
    (`BuildComponent.HidePreview` (`self.BP_BuildComponent`))
    (goto _label)))

(fn `UserConstructionScript`)